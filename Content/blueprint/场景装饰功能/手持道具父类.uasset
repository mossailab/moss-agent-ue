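; Parent Blueprint for handheld props (手持道具父类) that attach to a given component and carry NFT ID, wallet address and code data.
; BeginPlay hides the actor, passes its settings through a server set-variables event, then reveals it after a short delay.
; It then snaps to the parent component, sets its lifespan and runs optional delayed branches: physics simulation, timeline-lerped Arrow movement and detachment.
; Mesh collision is enabled early depending on product state.
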(event `服务器-设置变量`
  (params (`附加的组件` :type "SceneComponent Object Reference") (`生命周期` :type "Float (double-precision)") (`模拟物理延迟` :type "Float (double-precision)") (`移动偏移` :type "Transform Structure") (`移动延迟` :type "Float (double-precision)") (`移动速度` :type "Float (double-precision)") (`脱离附加延迟` :type "Float (double-precision)") (NFTid :type String) (`钱包地址` :type String) (code :type String))
  (set `self.附加的组件` `附加的组件`)
  (set `self.生命周期` `生命周期`)
  (set `self.模拟物理延迟` `模拟物理延迟`)
  (set `self.移动偏移` `移动偏移`)
  (set `self.移动延迟` `移动延迟`)
  (set `self.移动速度` `移动速度`)
  (set `self.脱离附加延迟` `脱离附加延迟`)
  (set `self.NFTid` NFTid)
  (set `self.钱包地址` `钱包地址`)
  (set `self.code` code))

(event `self.ReceiveBeginPlay`
  (bind `_脱离附加延迟` (`self.脱离附加延迟`))
  (bind `_模拟物理延迟` (`self.模拟物理延迟`))
  (bind _staticmesh (`self.StaticMesh`))
  (if (not (`|EnumEquality` (`self.商品状态`) "NewEnumerator0"))
    (`PrimitiveComponent.SetCollisionEnabled` (`self.StaticMesh`) "QueryAndPhysics"))
  (`self.SetActorHiddenInGame` true)
  (`self.服务器-设置变量` (`self.附加的组件`) (`self.生命周期`) (`self.模拟物理延迟`) (`self.移动偏移`) (`self.移动延迟`) (`self.移动速度`) (`self.脱离附加延迟`) (`self.NFTid`) (`self.钱包地址`) (`self.code`))
  (`KismetSystemLibrary.Delay` 1.0)
  (`self.SetActorHiddenInGame` false)
  (`|ExecutionSequence`
    (:`then_0`
      (`self.SetLifeSpan` (`self.生命周期`))
      (`self.K2_AttachToComponent` (`self.附加的组件`) "None" "SnapToTarget" "SnapToTarget" "KeepRelative"))
    (:`then_1`
      (if (> `_模拟物理延迟` 0.0)
        (`KismetSystemLibrary.Delay` `_模拟物理延迟`)
        (`PrimitiveComponent.SetCollisionEnabled` _staticmesh "QueryAndPhysics")
        (`KismetSystemLibrary.Delay` 0.2)
        (`PrimitiveComponent.SetSimulatePhysics` _staticmesh true)))
    (:`then_2`
      (if (not (== (`self.移动速度`) 0.0))
        (`KismetSystemLibrary.Delay` (`self.移动延迟`))
        (set `self.初始变换` (`SceneComponent.GetRelativeTransform` (`self.Arrow`)))
        (`TimelineComponent.SetPlayRate` (`self.时间轴`) (`self.移动速度`))
        (bind (_direction `_新建轨道_0`) (`Timeline|时间轴` :!via `PlayFromStart`)
          (:`Update`
            (`SceneComponent.K2_SetRelativeTransform` (`self.Arrow`) (`KismetMathLibrary.TLerp` (`self.初始变换`) (`self.移动偏移`) `_新建轨道_0`) false false)))))
    (:`then_3`
      (if (> `_脱离附加延迟` 0.0)
        (`KismetSystemLibrary.Delay` `_脱离附加延迟`)
        (`self.K2_DetachFromActor` "KeepWorld" "KeepWorld" "KeepWorld")))))

(fn `UserConstructionScript`)