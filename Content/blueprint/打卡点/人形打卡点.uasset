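; Humanoid check-in point (人形打卡点) that wanders around its spawn point, then seeks out an Agent to trigger its mining-success effect.
; BeginPlay starts a random AI move loop, gated by 停止随机移动 (true allows wandering despite its name), and a looping Pawn sphere-trace timer.
; Finding a non-display Agent clears the timer for good and starts a chase, retried on failure.
; Success plays the effect, then resumes wandering without further detection.
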(event `self.ReceiveBeginPlay`
  (set `self.巡逻中心` (`self.K2_GetActorLocation`))
  (bind _returnvalue (`KismetSystemLibrary.K2_SetTimerDelegate` (delegate `自定义事件`) 1.0 true))
  (set `self.寻找玩家定时器` _returnvalue)
  (if (`self.停止随机移动`) :!label _label
    (`|AIMoveTo` self (`NavigationSystemV1.K2_GetRandomReachablePointInRadius` (`self.巡逻中心`) 3000.0 null null) null
      (:`then`
        (`KismetSystemLibrary.Delay` (`KismetMathLibrary.RandomFloatInRange` 2.0 12.0))
        (goto _label)))))

(event `自定义事件`
  (bind _returnvalue (`self.K2_GetActorLocation`))
  (bind `_发现的agent` (`self.发现的Agent`))
  (bind _outhit (`KismetSystemLibrary.SphereTraceSingleForObjects` :`Start` _returnvalue :`End` _returnvalue :`Radius` 3000.0 :`ObjectTypes` (`|MakeArray` "ObjectTypeQuery3" :!type "EObjectTypeQuery Enum") :`DrawDebugType` "ForDuration"))
  (bind _asagent (cast `/Game/Game/Agent` (`.HitActor` (`GameplayStatics.BreakHitResult` _outhit))))
  (if (not (`/Game/Game/Agent.为商品展示` _asagent))
    (set `self.发现的Agent` _asagent)
    (set `self.停止随机移动` false)
    (`KismetSystemLibrary.K2_ClearAndInvalidateTimerHandle` (`self.寻找玩家定时器`))
    (`|AIMoveTo` self (0.0 0.0 0.0) `_发现的agent` :!label _label_2
      (:`OnSuccess`
        (`/Game/Game/Agent.挖矿成功效果` `_发现的agent`)
        (`KismetSystemLibrary.Delay` 2.0)
        (set `self.停止随机移动` true)
        (goto _label))
      (:`OnFail`
        (`KismetSystemLibrary.Delay` 1.0)
        (goto _label_2)))))

(fn `UserConstructionScript`)