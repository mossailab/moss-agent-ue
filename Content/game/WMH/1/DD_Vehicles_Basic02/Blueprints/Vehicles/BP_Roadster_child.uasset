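; Roadster vehicle Blueprint, a child class that adds configurable body parts to its parent.
; After the parent construction script runs, it sets visibility on two skirt meshes, a spoiler and a hard top from matching boolean variables.
; The event graph holds only disabled default events, so the child adds no runtime logic of its own.
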(fn `UserConstructionScript`
  (`parent.UserConstructionScript`)
  (`SceneComponent.SetVisibility` (`self.skirt1_mesh`) (`self.skirt1`) false)
  (`SceneComponent.SetVisibility` (`self.skirt2_mesh`) (`self.skirt2`) false)
  (`SceneComponent.SetVisibility` (`self.spoiler_mesh`) (`self.spoiler`) false)
  (`SceneComponent.SetVisibility` (`self.hard_top_mesh`) (`self.hard_top`) false))