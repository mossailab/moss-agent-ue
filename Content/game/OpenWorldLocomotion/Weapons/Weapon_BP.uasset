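; Base weapon Blueprint for the open-world locomotion system that mounts to a character mesh socket and computes its aim toward screen center.
; BeginPlay snaps the attachment to the parent mesh socket and caches whether the instigator is locally controlled.
; For locally controlled, aimable weapons, Tick interpolates WeaponRotation using a look-at from AimTarget to the Arrow component's location.
; The file only stores that rotation and does not apply it.
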(event `self.ReceiveBeginPlay`
  (bind _returnvalue (`self.GetInstigator`))
  (`self.K2_AttachToComponent` (`self.ParentMesh`) (`self.Socket Name`) "SnapToTarget" "SnapToTarget" "SnapToTarget" false)
  (`/Engine/EditorBlueprintResources/StandardMacros.IsValid` _returnvalue
    (:`Is Valid`
      (set `self.LocalyControlled` (`Pawn.IsLocallyControlled` _returnvalue)))))

(event `self.ReceiveTick`
  (params (DeltaSeconds :type "Float (single-precision)"))
  ;[1 1 1] Logic used to point your weapon at the location in the middle of the screen
  (if (and (`self.LocalyControlled`) (`self.CanBeAimed`))
    (set `self.WeaponRotation` (`KismetMathLibrary.RInterpTo` (`self.WeaponRotation`) (`KismetMathLibrary.FindLookAtRotation` (`self.AimTarget`) (`SceneComponent.K2_GetComponentLocation` (`self.Arrow`))) (`GameplayStatics.GetWorldDeltaSeconds`) 50.0))))

(fn `UserConstructionScript`)