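; Networked Open World Locomotion character component that manages animation overlays defined by OverlayData, including activation, aiming and combat stance.
; Activation plays class-matched pull-out or put-away montages, replicated through server and multicast events, while locomotion state and sliding gate whether the overlay stays enabled.
; RepNotifies push overlay and aim changes to the character and base component, driving stance, rotation lock and climbing/gliding restrictions.
; Tick updates hip rotation and times out combat stance.
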(event `ActivateOverlay_Event`
  (params (OverlayActive :type Boolean))
  (bind _overlaydata (`self.OverlayData`))
  ;[1 1 1] ActivateOverlay
  (`self.OverlayData`
    (:`then`
      (set `self.OverlayActive` OverlayActive)
      (bind _returnvalue (`AnimInstance.Montage_Play` (`SkeletalMeshComponent.GetAnimInstance` (`Character.Mesh` (`self.Character`))) (select `bool` (`self.OverlayActive`) :`false` (`self.FindAnimMontage` (`/Game/game/OpenWorldLocomotion/Data/DataAsset/AnimOverlay_PDA.PutAwayAnim` _overlaydata)) :`true` (`self.FindAnimMontage` (`/Game/game/OpenWorldLocomotion/Data/DataAsset/AnimOverlay_PDA.PullOutAnim` _overlaydata))) 1.0 "Duration" 0.0 true))
      (if (`self.OverlayActive`)
        (set `self.OverlayEnabled` true)
        (else
          (set `self.Aiming` false)
          (`self.SetCombatStance` false)
          (`KismetSystemLibrary.Delay` _returnvalue)
          (set `self.OverlayEnabled` false))))
    (:`else`
      (set `self.OverlayActive` false)
      (set `self.OverlayEnabled` false))))

(event `self.ReceiveBeginPlay`
  ;[1 0 1] Initialize component
  (`parent.ReceiveBeginPlay`)
  (add `/Game/game/OpenWorldLocomotion/CharacterComponents/基础部分.ChangeLocomotionState` (`self.BaseComponent`) (`|CreateDelegate` :!event `ChangeLocomotionState_Event`))
  (add `/Game/game/OpenWorldLocomotion/CharacterComponents/基础部分.DisableClimbing_Override` (`self.BaseComponent`) (`|CreateDelegate` :!event `DisableClimbing_Override_Event`)))

(event `ChangeLocomotionState_Event`
  (params (NewLocomotionState :type "/Game/game/OpenWorldLocomotion/Data/Enum/E_LocomotionStates Enum" :default "NewEnumerator0") (PrevLocomotionState :type "/Game/game/OpenWorldLocomotion/Data/Enum/E_LocomotionStates Enum" :default "NewEnumerator0"))
  ;[1 1 0] ChangeLocomotionState
  (if (`self.OverlayActive`)
    (set `self.OverlayEnabled` (`BlueprintMapLibrary.Map_Find` (`self.OverlayEnabledForLocomotionState`) NewLocomotionState))))

(event `OverlayEnabled_SERVER`
  (params (Enabled :type Boolean))
  ;[1 1 1] OverlayEnabled
  (set `self.OverlayEnabled` Enabled))

(event `Aiming_SERVER`
  (params (Aiming :type Boolean))
  ;[1 1 1] Aiming
  (set `self.Aiming` Aiming))

(event `SwitchOverlay_SERVER`
  (params (OverlayData :type "/Game/game/OpenWorldLocomotion/Data/DataAsset/AnimOverlay_PDA Object Reference"))
  ;[1 1 1] SwitchOverlay
  (set `self.OverlayData` OverlayData))

(event `ActivateOverlay_SERVER`
  (params (OverlayActive :type Boolean))
  ;[1 1 1] ActivateOverlay
  (`self.ActivateOverlay_MULTICAST` OverlayActive))

(event `ActivateOverlay_MULTICAST`
  (params (OverlayActive :type Boolean))
  ;[1 1 1] ActivateOverlay
  (if (not (`Pawn.IsLocallyControlled` (`self.Character`)))
    (`self.ActivateOverlay_Event` OverlayActive)))

(event `self.ReceiveTick`
  (params (DeltaSeconds :type "Float (single-precision)"))
  (`parent.ReceiveTick` DeltaSeconds)
  (`self.SetHipRotation`)
  (if (and (`/Game/game/OpenWorldLocomotion/CharacterComponents/基础部分.CombatStance` (`self.BaseComponent`)) (>= (`self.DisableCombatStanceDelay`) 0.0))
    (if (`KismetMathLibrary.BooleanNAND` (`self.DisableCombatStanceOnlyWhenStatic`) (not (`KismetMathLibrary.Vector_IsZero` (`Actor.GetVelocity` (`self.Character`)))) (`self.Aiming`))
      (`KismetSystemLibrary.RetriggerableDelay` (`self.DisableCombatStanceDelay`))
      (`self.SetCombatStance` false)))
  (if (`self.OverlayActive`)
    (if (`self.DisableOverlayWhenSliding`)
      (if (`/Game/game/OpenWorldLocomotion/CharacterComponents/基础部分.IsSliding` (`self.BaseComponent`))
        (set `self.OverlayEnabled` false)
        (elif (not (`self.OverlayEnabled`))
          (set `self.OverlayEnabled` (`BlueprintMapLibrary.Map_Find` (`self.OverlayEnabledForLocomotionState`) (`/Game/game/OpenWorldLocomotion/CharacterComponents/基础部分.LocomotionState` (`self.BaseComponent`)))))))))

(fn `ActivateOverlay`
  (params (OverlayActive :type Boolean))
  (`self.ActivateOverlay_Event` OverlayActive)
  (if (not (`KismetSystemLibrary.IsStandalone`))
    (`self.ActivateOverlay_SERVER` OverlayActive)))

(fn `Aim`
  (params (Aim :type Boolean))
  (if (`self.OverlayEnabled`)
    (bind _overlaydata (`self.OverlayData`)
      (:`then`
        (if (`/Game/game/OpenWorldLocomotion/Data/DataAsset/AnimOverlay_PDA.CanBeAimed` _overlaydata)
          (set `self.Aiming` Aim)
          (`|ExecutionSequence` :!label _label
            (:`then_0`
              ;[1 1 1] Disables climbing or/and gliding while aiming (controled through variables)
              (if (or (`self.Aiming_DisableClimbing`) (`self.Aiming_MantleOnly`))
                (`/Game/game/OpenWorldLocomotion/CharacterComponents/基础部分.DisableClimbing_Override` (`self.BaseComponent`) (and (`self.Aiming`) (`self.Aiming_DisableClimbing`)) (and (`self.Aiming`) (`self.Aiming_MantleOnly`))))
              (if (`self.Aiming_DisableGliding`)
                (`/Game/game/OpenWorldLocomotion/CharacterComponents/基础部分.DisableGliding_Override` (`self.BaseComponent`) (`self.Aiming`))))
            (:`then_1`
              (if (not (`Actor.HasAuthority` (`self.Character`)))
                (`self.Aiming_SERVER` (`self.Aiming`)))))
          (else
            (if (`self.Aiming`) :!label _label_2
              (set `self.Aiming` false)
              (goto _label)))))
      (:`else`
        (goto _label_2)))
    (else
      (goto _label_2))))

(fn `DisableClimbing_Override_Event`
  (params (DisableClimbing :type Boolean) (MantleOnly :type Boolean))
  (if (or (`self.OverlayEnabled_DisableClimbing`) (`self.OverlayEnabled_MantleOnly`))
    (if DisableClimbing
      _
      (elif (and (`self.OverlayEnabled`) (`self.OverlayEnabled_DisableClimbing`))
        (`/Game/game/OpenWorldLocomotion/CharacterComponents/基础部分.DisableClimbing_Override` (`self.BaseComponent`) (and (`self.OverlayEnabled`) (`self.OverlayEnabled_DisableClimbing`)) (and (`self.OverlayEnabled`) (`self.OverlayEnabled_MantleOnly`)) :!label _label)
        (elif MantleOnly
          _
          (elif (and (`self.OverlayEnabled`) (`self.OverlayEnabled_MantleOnly`))
            (goto _label)))))))

(fn `FindAnimMontage`
  (params (InputPin :type "Map of Character Class Reference to AnimMontage Object Reference"))
  (returns (Montage :type "AnimMontage Object Reference"))
  (bind _returnvalue (`GameplayStatics.GetObjectClass` (`self.Character`)))
  (bind (_value _returnvalue_2) (`BlueprintMapLibrary.Map_Find` InputPin _returnvalue))
  (if _returnvalue_2
    (return _value)
    (else
      (bind _keys (`BlueprintMapLibrary.Map_Keys` InputPin))
      (for _array_element _keys
        (if (`KismetMathLibrary.ClassIsChildOf` _returnvalue _array_element)
          (return (`BlueprintMapLibrary.Map_Find` InputPin _array_element))))
      (return null))))

(fn `GetData`
  (returns (OverlayEnabled :type Boolean) (OverlayActive :type Boolean) (Aiming :type Boolean) (OverlayData :type "/Game/game/OpenWorldLocomotion/Data/DataAsset/AnimOverlay_PDA Object Reference"))
  (return (`self.OverlayEnabled`) (`self.OverlayActive`) (`self.Aiming`) (`self.OverlayData`)))

(fn `Input_ActivateOverlay`
  (bind _returnvalue (not (`self.OverlayActive`)))
  (if (`|EnumEquality` (`/Game/game/OpenWorldLocomotion/CharacterComponents/基础部分.LocomotionState` (`self.BaseComponent`)) "NewEnumerator1")
    (if (not (`KismetSystemLibrary.IsStandalone`))
      (`self.ActivateOverlay_SERVER` _returnvalue))
    (`self.ActivateOverlay_Event` _returnvalue)))

(fn `OnRep_Aiming`
  (message `/Game/game/OpenWorldLocomotion/Data/OWL_Interface_BPI.BPI_IsAiming` (`self.Character`) (`self.Aiming`))
  (`/Game/game/OpenWorldLocomotion/CharacterComponents/基础部分.OnAimingChange` (`self.BaseComponent`) (`self.Aiming`))
  (if (`self.Aiming`)
    (`self.SetCombatStance` true)
    (`/Game/game/OpenWorldLocomotion/CharacterComponents/基础部分.Switch Rotation Mode` (`self.BaseComponent`) "NewEnumerator1"))
  (set `/Game/game/OpenWorldLocomotion/CharacterComponents/基础部分.LockRotationMode` (`self.Aiming`) (`self.BaseComponent`)))

(fn `OnRep_OverlayData`
  (`/Engine/EditorBlueprintResources/StandardMacros.IsValid` (`self.OverlayData`)
    (:`Is Valid`
      (set `self.DisableCombatStanceDelay` (`/Game/game/OpenWorldLocomotion/Data/DataAsset/AnimOverlay_PDA.DisableCombatStanceDelay` (`self.OverlayData`)))
      (set `self.DisableCombatStanceOnlyWhenStatic` (`/Game/game/OpenWorldLocomotion/Data/DataAsset/AnimOverlay_PDA.DisableCombatStanceOnlyWhenStatic` (`self.OverlayData`)))
      (if (`self.OverlayEnabled`)
        (set `self.OverlayEnabled` false)
        (set `self.OverlayEnabled` true)))
    (:`Is Not Valid`
      (set `self.OverlayEnabled` false)
      (`self.SetCombatStance` false)
      (set `self.OverlayActive` false)
      (set `self.Aiming` false))))

(fn `OnRep_OverlayEnabled`
  (message `/Game/game/OpenWorldLocomotion/Data/OWL_Interface_BPI.BPI_OnOverlayEnabled` (`self.Character`) (`self.OverlayEnabled`))
  (`|ExecutionSequence`
    (:`then_0`
      ;[1 1 1] Disables climbing or/and gliding when overlay is enabled (controled through variables)
      (if (or (`self.OverlayEnabled_DisableClimbing`) (`self.OverlayEnabled_MantleOnly`))
        (`/Game/game/OpenWorldLocomotion/CharacterComponents/基础部分.DisableClimbing_Override` (`self.BaseComponent`) (and (`self.OverlayEnabled`) (`self.OverlayEnabled_DisableClimbing`)) (and (`self.OverlayEnabled`) (`self.OverlayEnabled_MantleOnly`))))
      (if (`self.OverlayEnabled_DisableGliding`)
        (`/Game/game/OpenWorldLocomotion/CharacterComponents/基础部分.DisableGliding_Override` (`self.BaseComponent`) (`self.OverlayEnabled`))))
    (:`then_1`
      (if (`self.OverlayEnabled`)
        (bind _overlaydata (`self.OverlayData`)
          (:`then`
            (`self.SetCombatStance` (`/Game/game/OpenWorldLocomotion/Data/DataAsset/AnimOverlay_PDA.CombatStanceOnOverlayEnabled` _overlaydata)))
          (:`else`))))))

(fn `SetCombatStance`
  (params (CombatStance :type Boolean))
  (bind _output_get (set `/Game/game/OpenWorldLocomotion/CharacterComponents/基础部分.CombatStance` CombatStance (`self.BaseComponent`)))
  (`/Game/game/OpenWorldLocomotion/CharacterComponents/基础部分.OnStanceChanged` (`self.BaseComponent`) _output_get))

(fn `SetHipRotation`
  (bind _basecomponent (`self.BaseComponent`))
  (bind _overlaydata (`self.OverlayData`))
  (if (and (`self.OverlayEnabled`) (`KismetSystemLibrary.IsValid` _overlaydata))
    (set `/Game/game/OpenWorldLocomotion/CharacterComponents/基础部分.HipRotation` (select `bool` (`/Game/game/OpenWorldLocomotion/CharacterComponents/基础部分.CombatStance` (`self.BaseComponent`)) :`false` (`/Game/game/OpenWorldLocomotion/Data/DataAsset/AnimOverlay_PDA.HipRotation_Relaxed` _overlaydata) :`true` (`/Game/game/OpenWorldLocomotion/Data/DataAsset/AnimOverlay_PDA.HipRotation_Combat` _overlaydata)) _basecomponent)
    (else
      (set `/Game/game/OpenWorldLocomotion/CharacterComponents/基础部分.HipRotation` "NewEnumerator0" _basecomponent))))

(fn `Switch Overlay`
  (params (OverlayData :type "/Game/game/OpenWorldLocomotion/Data/DataAsset/AnimOverlay_PDA Object Reference"))
  (set `self.OverlayData` OverlayData)
  (if (`Actor.HasAuthority` (`self.Character`))
    _))