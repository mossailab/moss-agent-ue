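; BP_Placable is a replicated placeable actor whose static mesh shows one of three textures chosen by TextureIndex.
; On BeginPlay with authority, or on LoadActorState, it creates a dynamic instance of M_Placable, sets the texture from IndexToTexture and forces a net update.
; OnRep_TextureIndex repeats the material setup when the index replicates, keeping clients visually in sync.
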(event `self.ReceiveBeginPlay`
  (`/Engine/EditorBlueprintResources/ActorMacros.Switch Has Authority`
    (:`Authority`
      (bind _returnvalue (`PrimitiveComponent.CreateDynamicMaterialInstance` (`self.StaticMesh`) 0 "/Game/game/AAA/BPs/M_Placable.M_Placable" "None" :!label _label))
      (`MaterialInstanceDynamic.SetTextureParameterValue` _returnvalue "Texture" (`self.IndexToTexture` (`self.TextureIndex`)))
      (`self.ForceNetUpdate`))))

(event `self.LoadActorState`
  (goto _label))

(fn `IndexToTexture`
  (params (Index :type Integer))
  (returns (text :type "Texture2D Object Reference"))
  (return (select `int` Index :`0` null :`1` null :`2` null :!type "Texture2D Object Reference")))

(fn `OnRep_TextureIndex`
  (bind _returnvalue (`PrimitiveComponent.CreateDynamicMaterialInstance` (`self.StaticMesh`) 0 "/Game/game/AAA/BPs/M_Placable.M_Placable" "None"))
  (`MaterialInstanceDynamic.SetTextureParameterValue` _returnvalue "Texture" (`self.IndexToTexture` (`self.TextureIndex`))))

(fn `UserConstructionScript`)