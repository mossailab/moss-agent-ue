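; Image_download is a short-lived Actor that downloads an image from a URL and hands it back as a texture.
; On BeginPlay it builds a save path from the 2D image folder and the link's file name and suffix, then downloads to it.
; On success, RuntimeImageLoader loads the file asynchronously and the 下载完成 dispatcher broadcasts the texture.
; The actor destroys itself after a short delay.
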(event `self.ReceiveBeginPlay`
  (bind `_链接` (`self.链接`))
  (bind (`_文件名` `_后缀`) (`/Game/game/函数库.链接转文件名` `_链接`))
  (bind _returnvalue (`KismetStringLibrary.Concat_StrStr` (`/Game/game/函数库.图片2d文件路径`) `_文件名` `_后缀`))
  (set `self.路径` _returnvalue)
  (`FileToStorageDownloader.DownloadFileToStorage` `_链接` _returnvalue 0.0 "" false (delegate `进度`) (delegate `结果`)))

(event `进度`
  (params (BytesReceived :type Integer64) (ContentLength :type Integer64) (ProgressRatio :type "Float (single-precision)")))

(event `结果`
  (params (Result :type "EDownloadToStorageResult Enum" :default "Success") (SavedPath :type String) (Downloader :type "FileToStorageDownloader Object Reference"))
  (if (`|EnumEquality` Result "Success")
    (bind _outtexture (`RuntimeImageLoader.LoadImageAsync` :`self` (subsystem `RuntimeImageLoader`) :`ImageFilename` (`self.路径`)))
    (`self.下载完成` _outtexture))
  (`KismetSystemLibrary.Delay` 1.0)
  (`self.K2_DestroyActor`))

(fn `UserConstructionScript`)