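; Placeable island/level marker actor with a streaming volume and an island-name display with its own sphere volume.
; The construction script reads the display-name prefix (YX, TP, YS) to pick a range that sizes both volumes, with a separate variable for streaming height.
; YX actors also get an enlarged name display.
; Non-island actors with a level name set destroy their name display and static mesh.
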(fn `UserConstructionScript`
  (bind _lefts (`KismetStringLibrary.Split` (`KismetSystemLibrary.GetDisplayName` self) "_"))
  (bind _returnvalue (== _lefts "YX"))
  (bind _returnvalue_2 (select `bool` _returnvalue :`false` (select `bool` (== _lefts "TP") :`false` (select `bool` (== _lefts "YS") :`false` 100000.0 :`true` (`self.YS范围`)) :`true` (`self.TP范围`)) :`true` (`self.YX范围`)))
  (bind _returnvalue_3 (/ _returnvalue_2 50.0))
  (`self.SetActorEnableCollision` true)
  (`SceneComponent.SetRelativeScale3D` (`self.流送体积`) (`KismetMathLibrary.MakeVector` _returnvalue_3 _returnvalue_3 (`self.Z高度`)))
  (`SphereComponent.SetSphereRadius` (`self.岛名显示体积`) _returnvalue_2 true)
  (if _returnvalue
    (`SceneComponent.SetRelativeScale3D` (`self.岛名显示`) (200.0 200.0 200.0)))
  (if (`self.是否为岛屿`)
    _
    (elif (not (`KismetStringLibrary.IsEmpty` (`self.关卡名称`)))
      (`ActorComponent.K2_DestroyComponent` (`self.岛名显示`))
      (`ActorComponent.K2_DestroyComponent` (`self.StaticMesh`)))))