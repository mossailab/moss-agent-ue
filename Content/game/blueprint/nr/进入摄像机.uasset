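; Camera actor for the character-creation mode (捏人模式) that lets the player turn the preview model and zoom.
; While the left mouse button is held, the Turn axis, scaled by a speed variable, yaws the game mode's model actor.
; The mouse wheel plays or reverses a timeline that lerps spring-arm length, stopping shortly after wheel release.
; Rotation and zoom values are printed for debugging.
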(event `Key|LeftMouseButton`
  (params (Key :type "Key Structure"))
  (:`Pressed`
    (set `self.是否松开` false))
  (:`Released`
    (set `self.是否松开` true)))

(event `InputAxis|Turn`
  (params (AxisValue :type "Float (single-precision)"))
  (bind _returnvalue (* AxisValue (`self.速度`)))
  (bind `_模特` (`/Game/game/blueprint/nr/捏人模式.模特` (cast `/Game/game/blueprint/nr/捏人模式` (`GameplayStatics.GetGameMode`) :!pure true)))
  (bind (_returnvalue_roll _returnvalue_pitch _returnvalue_yaw) (`KismetMathLibrary.BreakRotator` (`self.K2_GetActorRotation` `_模特`)))
  (if (not (`self.是否松开`))
    (`KismetSystemLibrary.PrintString` (`KismetStringLibrary.Conv_DoubleToString` _returnvalue))
    (`self.K2_SetActorRotation` `_模特` (`KismetMathLibrary.MakeRotator` _returnvalue_roll _returnvalue_pitch (+ _returnvalue_yaw _returnvalue)) false)))

(event `self.ReceiveBeginPlay`)

(event `Key|MouseScrollUp`
  (params (Key :type "Key Structure"))
  (bind _springarm (`self.SpringArm`))
  (:`Pressed`
    (bind (_direction `_新建轨道_0`) (`Timeline|时间轴_0` :!via `Reverse` :!label _label)
      (:`Update`
        (`KismetSystemLibrary.PrintString` (`KismetStringLibrary.Conv_DoubleToString` (`SpringArmComponent.TargetArmLength` _springarm)))
        (set `SpringArmComponent.TargetArmLength` (`KismetMathLibrary.Lerp` 200.0 500.0 `_新建轨道_0`) _springarm))))
  (:`Released`
    (`KismetSystemLibrary.Delay` 0.2 :!label _label_2)
    (goto _label :!via `Stop`)))

(event `Key|MouseScrollDown`
  (params (Key :type "Key Structure"))
  (:`Pressed`
    (goto _label))
  (:`Released`
    (goto _label_2)))

(fn `UserConstructionScript`)