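; Placed glTF runtime asset actor representing a shop work, carrying its name, price, sale status, cover, shop and link data.
; On BeginPlay it sends IDs and token through a server event.
; After a random delay, authority destroys nearby same-ID duplicates, then fetches the work via VaRest and stores parsed JSON through another server event.
; Without a model link, the Cube becomes visible and remote instances texture it with the downloaded cover image.
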(event `self.ReceiveBeginPlay`
  (bind _returnvalue (`self.K2_GetActorLocation`))
  (bind _cube (`self.Cube`))
  (`parent.ReceiveBeginPlay`)
  (`KismetSystemLibrary.Delay` 0.2)
  (`self.服务器-ID` (`self.ID`) (`self.拥有者ID`) (`/Game/game/INS.令牌` (cast `/Game/game/INS` (`GameplayStatics.GetGameInstance`) :!pure true)) (`self.1155ID`) (`self.模型链接为空`))
  (`|ExecutionSequence`
    (:`then_0`
      (`/Engine/EditorBlueprintResources/ActorMacros.Switch Has Authority`
        (:`Authority`
          (`KismetSystemLibrary.Delay` (`KismetMathLibrary.RandomFloatInRange` 0.0 2.0))
          (bind _outhits (`KismetSystemLibrary.SphereTraceMultiForObjects` _returnvalue _returnvalue 10.0 (`|MakeArray` "ObjectTypeQuery2" :!type "EObjectTypeQuery Enum")))
          (for _array_element _outhits
            (bind _asmygl_tfruntime_asset_actor (cast `/Game/game/blueprint/Interactive_Object/MyglTFRuntimeAssetActor` (`.HitActor` (`GameplayStatics.BreakHitResult` _array_element))))
            (if (== (`/Game/game/blueprint/Interactive_Object/MyglTFRuntimeAssetActor.ID` _asmygl_tfruntime_asset_actor) (`self.ID`))
              (`self.K2_DestroyActor` _asmygl_tfruntime_asset_actor)))
          (if (> (`KismetStringLibrary.Conv_StringToInt` (`self.ID`)) 0)
            (set `self.属性json` (`|MakeJson`))
            (bind _returnvalue_2 (`VaRestSubsystem.ConstructVaRestRequestExt` (subsystem `VaRestSubsystem`) "GET" "x_www_form_urlencoded_url"))
            (`VaRestRequestJSON.SetHeader` _returnvalue_2 "X-Access-Token" (`self.令牌`))
            (`VaRestRequestJSON.ProcessURL` _returnvalue_2 (`/Game/game/函数库.附加区块链接口` (`KismetStringLibrary.Concat_StrStr` (`/Game/game/INS.API` (cast `/Game/game/INS` (`GameplayStatics.GetGameInstance`) :!pure true)) "works/works/queryById?id=" (`self.ID`) "&sellUserId=" (`self.拥有者ID`))))
            (add `VaRestRequestJSON.OnRequestComplete` _returnvalue_2 (delegate `链接结果`))))))
    (:`then_1`
      (`KismetSystemLibrary.Delay` 2.5)
      (if (`self.模型链接为空`)
        (`SceneComponent.SetVisibility` (`self.Cube`) true false)
        (`/Engine/EditorBlueprintResources/ActorMacros.Switch Has Authority`
          (:`Remote`
            (`SceneComponent.SetVisibility` _cube true false)
            (bind _returnvalue_3 (`PrimitiveComponent.CreateDynamicMaterialInstance` _cube 0 "/Game/ZY/材质/材质实例/画材质_Inst.画材质_Inst" "None"))
            (bind _texture (`/Game/game/蓝图宏库.图片下载` (`self.封面图链接`))
              (:`On Success`
                (`MaterialInstanceDynamic.SetTextureParameterValue` _returnvalue_3 "贴图" _texture)))))))))

(event `服务器-ID`
  (params (`自身ID` :type String) (`拥有者ID` :type String) (`令牌` :type String) (`1155ID` :type String) (`模型链接为空` :type Boolean))
  (set `self.ID` `自身ID`)
  (set `self.拥有者ID` `拥有者ID`)
  (set `self.令牌` `令牌`)
  (set `self.1155ID` `1155ID`)
  (set `self.模型链接为空` `模型链接为空`))

(event `链接结果`
  (params (Request :type "VaRestRequestJSON Object Reference"))
  (bind `_属性json` (`self.属性json`))
  (bind _returnvalue (`VaRestJsonObject.GetObjectField` `_属性json` "result"))
  (bind _returnvalue_2 (`VaRestJsonObject.GetObjectField` _returnvalue "islandShopWorks"))
  (bind _returnvalue_3 (`VaRestJsonObject.GetObjectField` _returnvalue_2 "islandShop"))
  (bind _returnvalue_4 (`VaRestRequestJSON.GetResponseContentAsString` Request false))
  (`VaRestJsonObject.DecodeJson` `_属性json` _returnvalue_4 false)
  (set `self.二维码链接` (`VaRestJsonObject.GetStringField` _returnvalue_2 "buyHref"))
  (set `self.物品名称` (`VaRestJsonObject.GetStringField` _returnvalue "name"))
  (set `self.封面图链接` (`VaRestJsonObject.GetStringField` _returnvalue "verticalCoverImage"))
  (set `self.是否上架` (== (`VaRestJsonObject.GetStringField` _returnvalue "sellStatus") "Y"))
  (set `self.价格` (`VaRestJsonObject.GetNumberField` _returnvalue_2 "price"))
  (set `self.商品ID` (`VaRestJsonObject.GetStringField` _returnvalue_2 "id"))
  (set `self.头像链接` (`VaRestJsonObject.GetStringField` _returnvalue "versionNumber"))
  (set `self.logo` (`VaRestJsonObject.GetStringField` _returnvalue_3 "logo"))
  (set `self.店铺名称` (`VaRestJsonObject.GetStringField` _returnvalue_3 "name"))
  (set `self.详情网页` (`VaRestJsonObject.GetStringField` _returnvalue_2 "description"))
  (set `self.属性json` null)
  (`self.服务器-设置信息` (`self.二维码链接`) (`self.物品名称`) (`self.封面图链接`) (`self.是否上架`) (`self.价格`) (`self.logo`) (`self.店铺名称`) (`self.商品ID`) (`self.头像链接`) (`self.详情网页`)))

(event `服务器-设置信息`
  (params (`二维码链接` :type String) (`物品名称` :type String) (`封面图链接` :type String) (`是否上架` :type Boolean) (`价格` :type "Float (double-precision)") (logo :type String) (`店铺名称` :type String) (`商品ID` :type String) (`头像链接` :type String) (`详情网页` :type String))
  (set `self.二维码链接` `二维码链接`)
  (set `self.物品名称` `物品名称`)
  (set `self.封面图链接` `封面图链接`)
  (set `self.是否上架` `是否上架`)
  (set `self.价格` `价格`)
  (set `self.商品ID` `商品ID`)
  (set `self.头像链接` `头像链接`)
  (set `self.logo` logo)
  (set `self.店铺名称` `店铺名称`)
  (set `self.详情网页` `详情网页`))

(fn `UserConstructionScript`)