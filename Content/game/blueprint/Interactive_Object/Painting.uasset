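; Interactive painting actor that displays a picture, streamed video or GIF from a saved link on two meshes.
; Pictures download into a shared dynamic material; GIFs are downloaded to disk once and reloaded from that cache, with IPFS link rewriting.
; Player overlap asks the PLAY controller for a video; the returned index selects the media player, material and sound source.
; A five-second distance poll pauses playback and re-arms the trigger when the player leaves.
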(event `self.初始化结构`
  (bind `_图片链接` (`self.图片链接`))
  (`parent.初始化结构`)
  (if (not (`KismetStringLibrary.IsEmpty` `_图片链接`))
    (`self.画初始化` `_图片链接` (`KismetMathLibrary.FTrunc` (`|GetArrayItem` (`self.浮点`))))))

(event `下载进度`
  (params (BytesReceived :type Integer64) (ContentLength :type Integer64) (ProgressRatio :type "Float (single-precision)")))

(event `self.ReceiveDestroyed`
  (bind `_播放器` (break `/Game/game/结构/媒体结构` (`|GetArrayItem` (`self.媒体结构`) (`self.视频索引`))))
  (`/Engine/EditorBlueprintResources/StandardMacros.IsValid` `_播放器`
    (:`Is Valid`
      (`MediaPlayer.Pause` `_播放器`)
      (bind `_音效组件` (`self.音效组件`)
        (:`then`
          (`ActorComponent.K2_DestroyComponent` `_音效组件`))
        (:`else`)))))

(event `下载结果`
  (params (Result :type "EDownloadToStorageResult Enum" :default "Success") (SavedPath :type String) (Downloader :type "FileToStorageDownloader Object Reference"))
  (bind (`_文件名` `_后缀`) (`/Game/game/函数库.链接转文件名` (`self.图片链接`)))
  (switch `EDownloadToStorageResult` Result
    (:`Success`
      (bind _outgiftexture (`RuntimeGifReader.LoadGIF` (`KismetStringLibrary.Concat_StrStr` (`/Game/game/函数库.获取gif路径`) `_文件名` `_后缀`) "TF_Bilinear" :!label _label)
        (:`OnSuccess`
          (`MaterialInstanceDynamic.SetTextureParameterValue` (`self.画动态材质实例`) "贴图" _outgiftexture))))))

(event `self.ReceiveBeginPlay`
  (bind (`_文件名` `_后缀`) (`/Game/game/函数库.链接转文件名` (`self.图片链接`)))
  (bind _returnvalue (`KismetStringLibrary.Concat_StrStr` (`/Game/game/函数库.获取gif路径`) `_文件名` `_后缀`))
  (`parent.ReceiveBeginPlay`)
  (`KismetSystemLibrary.Delay` 1.0)
  (switch `int` (`self.1图片2视频4GIF`)
    (:`4`
      (if (`.bIsValid` (break `FileSDKFileInfo` (`FileSDKBPLibrary.GetFileOrDirectoryInfo` _returnvalue)))
        (goto _label)
        (else
          (`FileToStorageDownloader.DownloadFileToStorage` (`/Game/game/函数库.IPFS链接替换` (`self.图片链接`)) _returnvalue 0.0 "application/json" false (delegate `下载进度`) (delegate `下载结果`)))))))

(event `self.ReceiveTick`
  (params (DeltaSeconds :type "Float (single-precision)")))

(event `self.视频播放范围.OnComponentBeginOverlap`
  (params (OverlappedComponent :type "PrimitiveComponent Object Reference") (OtherActor :type "Actor Object Reference") (OtherComp :type "PrimitiveComponent Object Reference") (OtherBodyIndex :type Integer) (bFromSweep :type Boolean) (SweepResult :type "HitResult Structure (by ref)"))
  (bind _returnvalue (`GameplayStatics.GetPlayerController` 0))
  ;[1 1 1] 在用
  ;;[1 1 1] 播放视频
  (if (== OtherActor (`Controller.K2_GetPawn` _returnvalue))
    (switch `int` (`self.1图片2视频4GIF`)
      (:`2`
        (`/Engine/EditorBlueprintResources/StandardMacros.DoOnce` false :!label _label_2
          (:`Completed`
            (`/Game/game/PLAY.设置画视频` (cast `/Game/game/PLAY` _returnvalue :!pure true) self)))))))

(event `返回结果`
  (params (`视频索引` :type Integer))
  (bind (`_output_播放器` `_output_媒体源` `_output_媒体纹理` `_output_材质实例`) (break `/Game/game/结构/媒体结构` (`|GetArrayItem` (`self.媒体结构`) (`self.视频索引`))))
  (bind (`_播放器` `_媒体源` `_媒体纹理` `_材质实例` `_流送媒体源`) (break `/Game/game/结构/媒体结构` (`|GetArrayItem` (`self.媒体结构`) (`self.视频索引`))))
  ;[1 1 1] 在用
  ;;[1 1 1] 播放视频
  (set `self.视频索引` `视频索引`)
  (`self.距离判断`)
  (`/Engine/EditorBlueprintResources/StandardMacros.IsValid` `_流送媒体源`
    (:`Is Valid`
      (set `StreamMediaSource.StreamUrl` (`/Game/game/函数库.IPFS链接替换` (`self.图片链接`)) `_流送媒体源`)
      (set `self.播放器` `_播放器`)
      (`MediaPlayer.OpenSource` `_播放器` `_流送媒体源`)
      (`PrimitiveComponent.SetMaterial` (`self.画`) 0 `_output_材质实例`)
      (`PrimitiveComponent.SetMaterial` (`self.画1`) 0 `_output_材质实例`)
      (bind `_音效组件` (`self.音效组件`)
        (:`then`
          (`MediaSoundComponent.SetMediaPlayer` `_音效组件` `_播放器`))
        (:`else`
          (bind _returnvalue (`AddComponent|NODE_AddMediaSoundComponent-0`))
          (set `self.音效组件` _returnvalue)
          (`MediaSoundComponent.SetMediaPlayer` _returnvalue `_播放器`))))))

(event `距离判断`
  ;[1 1 1] 在用
  ;;[1 1 1] 播放视频
  (if (> (`KismetMathLibrary.VSize` (- (`self.K2_GetActorLocation`) (`self.K2_GetActorLocation` (`Controller.K2_GetPawn` (`GameplayStatics.GetPlayerController` 0))))) 1200.0) :!label _label_3
    (`|ExecutionSequence`
      (:`then_0`
        (`MediaPlayer.Pause` (`self.播放器`)))
      (:`then_1`
        (goto _label_2 :!via `Reset`)))
    (else
      (`KismetSystemLibrary.Delay` 5.0)
      (goto _label_3))))

(event `画初始化`
  (params (`链接` :type String) (`1图片2视频3GIF` :type Integer))
  ;[1 1 1] 在用
  (set `self.图片链接` `链接`)
  (bind _output_get (set `self.1图片2视频4GIF` `1图片2视频3GIF`))
  (`KismetArrayLibrary.Array_Set` (`self.浮点`) 0 (`KismetMathLibrary.Conv_IntToDouble` _output_get) true)
  (`KismetArrayLibrary.Array_Set` (`self.Tags`) 1 (`KismetSystemLibrary.MakeLiteralName` (select `int` `1图片2视频3GIF` :`0` "None" :`1` "picture" :`2` "video" :`3` "GIF" :!type "Name")) true)
  (switch `int` `1图片2视频3GIF`
    (:`1`
      (bind _texture (`/Game/game/蓝图宏库.图片下载` (`self.图片链接`))
        (:`On Success`
          (`MaterialInstanceDynamic.SetTextureParameterValue` (`self.画动态材质实例`) "贴图" _texture))))))

(fn `UserConstructionScript`
  (`parent.UserConstructionScript`)
  (bind _returnvalue (`PrimitiveComponent.CreateDynamicMaterialInstance` (`self.画`) 0 "/Game/ZY/材质/材质实例/画材质_Inst.画材质_Inst" "None"))
  (bind _output_get (set `self.画动态材质实例` _returnvalue))
  (`PrimitiveComponent.SetMaterial` (`self.画1`) 0 _output_get))