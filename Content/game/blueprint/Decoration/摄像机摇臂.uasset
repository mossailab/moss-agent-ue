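; Camera boom actor (摄像机摇臂) that rotates a spring arm from the local player's view input.
; On BeginPlay it attaches to a given actor through a server event and multicast, keeping world transform.
; Tick adds view X/Y input, read through a 默认角色 reference, to arm pitch (inverted) and yaw, zeroing roll.
; A range-checked event stores a zoom multiplier, and axis events store movement input; neither is applied here.
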(event `self.ReceiveBeginPlay`
  (`self.服务器-附加` (`self.附加的actor`)))

(event `服务器-附加`
  (params (ParentActor :type "Actor Object Reference"))
  (`self.组播-附加` ParentActor))

(event `组播-附加`
  (params (ParentActor :type "Actor Object Reference"))
  (`self.K2_AttachToActor` ParentActor "None" "KeepWorld" "KeepWorld" "KeepWorld"))

(event `self.ReceiveTick`
  (params (DeltaSeconds :type "Float (single-precision)"))
  (bind `_弹簧臂` (`self.弹簧臂`))
  (bind _returnvalue (`Controller.K2_GetPawn` (`GameplayStatics.GetPlayerController` 0)))
  (bind _returnvalue_2 (`SceneComponent.GetRelativeTransform` `_弹簧臂`))
  (cast `/Game/game/玩家` _returnvalue
    (:`then`
      _)
    (:`CastFailed`
      (bind `_as默认角色` (cast `/Game/game/默认角色` _returnvalue))))
  (set `self.视角 X输入` (`/Game/game/默认角色.视角X输入` `_as默认角色`))
  (set `self.视角 Y输入` (`/Game/game/默认角色.视角Y输入` `_as默认角色`))
  (`SceneComponent.K2_SetRelativeRotation` `_弹簧臂` (`KismetMathLibrary.MakeRotator` 0.0 (+ (* (`self.视角 X输入`) -1.0) (.pitch (.rotation _returnvalue_2))) (+ (`self.视角 Y输入`) (.yaw (.rotation _returnvalue_2)))) false false))

(event `视角缩放`
  (params (`值` :type "Float (double-precision)"))
  (if (`KismetMathLibrary.InRange_FloatFloat` (+ (* `值` 0.1) (`self.弹簧臂缩放倍数`)) 1.0 10.0)
    (set `self.弹簧臂缩放倍数` `值`)))

(event `InputAxis|MoveForward`
  (params (AxisValue :type "Float (single-precision)"))
  (set `self.移动输入Y` AxisValue))

(event `InputAxis|MoveRight`
  (params (AxisValue :type "Float (single-precision)"))
  (set `self.移动输入X` AxisValue))

(fn `UserConstructionScript`)