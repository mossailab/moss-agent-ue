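; Decoration actor that displays a thin line through a spline, tracking world positions A and B.
; The construction script adds two spline mesh segments along the spline points and stores them in an array.
; Every Tick moves the first two spline points to A and B, then refits each stored segment to the spline and sets a slightly thicker scale than at construction.
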(event `self.ReceiveTick`
  (params (DeltaSeconds :type "Float (single-precision)"))
  (bind _spline (`self.Spline`))
  (bind _spline_2 (`self.Spline`))
  (`SplineComponent.SetLocationAtSplinePoint` _spline 0 (`self.A`) "World" true)
  (`SplineComponent.SetLocationAtSplinePoint` _spline 1 (`self.B`) "World" true)
  (for (_array_element _array_index) (`self.样条网格体`)
    (bind (_location _tangent) (`SplineComponent.GetLocationAndTangentAtSplinePoint` _spline_2 _array_index "Local"))
    (bind (_location_2 _tangent_2) (`SplineComponent.GetLocationAndTangentAtSplinePoint` _spline_2 (+ _array_index 1) "Local"))
    (`SplineMeshComponent.SetStartAndEnd` _array_element _location _tangent _location_2 _tangent_2 true)
    (`SplineMeshComponent.SetStartScale` _array_element (0.05 0.05) true)
    (`SplineMeshComponent.SetEndScale` _array_element (0.05 0.05) true)))

(fn `UserConstructionScript`
  (bind _spline (`self.Spline`))
  (for _index (range 1 3)
    (bind _returnvalue (`AddComponent|NODE_AddSplineMeshComponent-0`))
    (bind (_location _tangent) (`SplineComponent.GetLocationAndTangentAtSplinePoint` _spline (- _index 1) "Local"))
    (bind (_location_2 _tangent_2) (`SplineComponent.GetLocationAndTangentAtSplinePoint` _spline _index "Local"))
    (`SplineMeshComponent.SetStartAndEnd` _returnvalue _location _tangent _location_2 _tangent_2 true)
    (`SplineMeshComponent.SetStartScale` _returnvalue (0.02 0.02) true)
    (`SplineMeshComponent.SetEndScale` _returnvalue (0.02 0.02) true)
    (`KismetArrayLibrary.Array_Add` (`self.样条网格体`) _returnvalue)))