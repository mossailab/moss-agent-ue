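; 超级尘埃 ("super dust") is a decoration actor that moves back and forth between two offsets from its starting location.
; On BeginPlay it caches that location and starts a timeline at the 速度 (speed) play rate.
; The timeline track lerps between the location plus A and plus B, setting the position without sweep.
; Each finish flips the playback direction, creating an endless ping-pong without using Tick.
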(event `self.ReceiveBeginPlay`
  (bind `_初始位置` (`self.初始位置`))
  (set `self.初始位置` (`self.K2_GetActorLocation`))
  (`TimelineComponent.SetPlayRate` (`self.时间轴`) (`self.速度`))
  (bind (_direction `_新建轨道_0`) (`Timeline|时间轴` :!via `PlayFromStart` :!label _label)
    (:`Update`
      (`self.K2_SetActorLocation` (`KismetMathLibrary.VLerp` (+ `_初始位置` (`self.A`)) (+ `_初始位置` (`self.B`)) `_新建轨道_0`)))
    (:`Finished`
      (if (`|EnumEquality` _direction "Forward")
        (goto _label :!via `ReverseFromEnd`)
        (else
          (goto _label :!via `PlayFromStart`))))))

(fn `UserConstructionScript`)