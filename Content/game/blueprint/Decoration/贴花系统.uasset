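; Decal decoration actor that displays a configurable material with a settable texture and color.
; An init event, run at construction and again one second after BeginPlay, applies the material and creates a dynamic instance carrying the texture and color parameters.
; Events swap the decal material or texture; texture changes update the local instance, then call a server-named event that stores the texture variable.
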(event `self.ReceiveBeginPlay`
  (`KismetSystemLibrary.Delay` 1.0)
  (`self.贴花初始化`))

(event `贴花初始化`
  (bind _decal (`self.Decal`))
  (bind `_动态材质` (`self.动态材质`))
  (`DecalComponent.SetDecalMaterial` _decal (`self.贴花材质`))
  (bind _returnvalue (`DecalComponent.CreateDynamicMaterialInstance` _decal))
  (set `self.动态材质` _returnvalue)
  (`MaterialInstanceDynamic.SetTextureParameterValue` `_动态材质` "纹理" (`self.纹理`))
  (`MaterialInstanceDynamic.SetVectorParameterValue` `_动态材质` "颜色" (`self.颜色`)))

(event `设置贴花`
  (params (NewDecalMaterial :type "MaterialInterface Object Reference"))
  (`DecalComponent.SetDecalMaterial` (`self.Decal`) NewDecalMaterial))

(event `设置贴图`
  (params (Value :type "Texture Object Reference"))
  (`MaterialInstanceDynamic.SetTextureParameterValue` (`self.动态材质`) "纹理" Value)
  (`self.服务器-设置贴图` Value))

(event `服务器-设置贴图`
  (params (`纹理` :type "Texture Object Reference"))
  (set `self.纹理` `纹理`))

(fn `UserConstructionScript`
  (`self.贴花初始化`))