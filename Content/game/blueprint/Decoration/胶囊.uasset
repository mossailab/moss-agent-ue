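; Decorative capsule (胶囊) actor that animates its static mesh in an endless loop from BeginPlay.
; A sped-up timeline lerps the mesh's relative location between the origin and an offset along its negative right vector, computed once at start.
; Each time the timeline finishes it restarts, occasionally after a short random-chance delay to break up the rhythm.
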(event `self.ReceiveBeginPlay`
  (set `self.NewVar_0` (* (`SceneComponent.GetRightVector` (`self.StaticMesh`)) -200.0))
  (`TimelineComponent.SetPlayRate` (`self.时间轴`) 6.0)
  (bind (_direction `_新建轨道_0`) (`Timeline|时间轴` :!via `PlayFromStart` :!label _label)
    (:`Update`
      (`SceneComponent.K2_SetRelativeLocation` (`self.StaticMesh`) (`KismetMathLibrary.VLerp` (0.0 0.0 0.0) (`self.NewVar_0`) `_新建轨道_0`) false false))
    (:`Finished`
      (if (> (`KismetMathLibrary.RandomIntegerInRange` 1 10) 8)
        (`KismetSystemLibrary.Delay` 0.2)
        (goto _label :!via `PlayFromStart`)
        (else
          (goto _label :!via `PlayFromStart`))))))

(fn `UserConstructionScript`)