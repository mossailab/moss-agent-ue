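; Voting display actor that shows one artwork's cover, name, token ID and vote count from the web API, picked by index.
; Clients fetch the list via VaRest after a random delay and load the cover into a dynamic material.
; Local player overlap casts a token-authenticated vote with a two-second cooldown, then refreshes the count and spawns any awarded badge through the player controller.
; The 3D count text scales up with votes, capped.
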(event `self.ReceiveBeginPlay`
  (`/Engine/EditorBlueprintResources/ActorMacros.Switch Has Authority`
    (:`Remote`
      (`KismetSystemLibrary.Delay` (`KismetMathLibrary.RandomFloatInRange` 5.0 20.0))
      (bind _output_get (set `self.Json投票` (`|MakeJson`)))
      (`VaRestSubsystem.CallURL` (subsystem `VaRestSubsystem`) (`KismetStringLibrary.Concat_StrStr` (`/Game/game/INS.API` (cast `/Game/game/INS` (`GameplayStatics.GetGameInstance`) :!pure true)) "works/voteWorks/list?pageSize=-1&currDrop=true") "GET" "x_www_form_urlencoded_url" _output_get (delegate `获取场景视频链接`)))))

(event `获取场景视频链接`
  (params (Request :type "VaRestRequestJSON Object Reference"))
  (bind `_json投票` (`self.Json投票`))
  (bind _output (`|GetArrayItem` (`VaRestJsonObject.GetObjectArrayField` (`VaRestJsonObject.GetObjectField` `_json投票` "result") "records") (`self.索引`)))
  (bind _returnvalue (`VaRestJsonObject.GetObjectField` _output "works"))
  (bind _returnvalue_2 (`VaRestRequestJSON.GetResponseContentAsString` Request false))
  (`VaRestJsonObject.DecodeJson` `_json投票` _returnvalue_2 false)
  (`/Engine/EditorBlueprintResources/StandardMacros.IsValid` _output
    (:`Is Valid`
      (set `self.id` (`VaRestJsonObject.GetStringField` _output "id"))
      (set `self.图片链接` (`VaRestJsonObject.GetStringField` _returnvalue "horizontalCoverImage"))
      (set `self.票数` (`VaRestJsonObject.GetIntegerField` _output "voteNum"))
      (set `Text3DComponent.Text` (`|FormatText` "ID:{0}" (`KismetTextLibrary.Conv_StringToText` (`VaRestJsonObject.GetStringField` _returnvalue "tokenId"))) (`self.seed`))
      (set `Text3DComponent.Text` (`KismetTextLibrary.Conv_StringToText` (`VaRestJsonObject.GetStringField` _returnvalue "name")) (`self.名称`))
      (`self.票数增加`)
      (bind _returnvalue_3 (`PrimitiveComponent.CreateDynamicMaterialInstance` (`self.Plane`) 0 "/Game/game/Material/母材质/普通母材质/水母材质.水母材质" "None"))
      (set `self.动态材质` _returnvalue_3)
      (bind _texture (`/Game/game/蓝图宏库.图片下载` (`self.图片链接`))
        (:`On Success`
          (`MaterialInstanceDynamic.SetTextureParameterValue` (`self.动态材质`) "纹理" _texture))))))

(event `获取票数`
  (bind _output_get (set `self.Json投票` (`|MakeJson`)))
  (`VaRestSubsystem.CallURL` (subsystem `VaRestSubsystem`) (`KismetStringLibrary.Concat_StrStr` (`/Game/game/INS.API` (cast `/Game/game/INS` (`GameplayStatics.GetGameInstance`) :!pure true)) "works/voteWorks/list?pageSize=-1&currDrop=true") "GET" "x_www_form_urlencoded_url" _output_get (delegate `1`)))

(event `self.Box.OnComponentBeginOverlap`
  (params (OverlappedComponent :type "PrimitiveComponent Object Reference") (OtherActor :type "Actor Object Reference") (OtherComp :type "PrimitiveComponent Object Reference") (OtherBodyIndex :type Integer) (bFromSweep :type Boolean) (SweepResult :type "HitResult Structure (by ref)"))
  (bind `_as玩家` (cast `/Game/game/玩家` OtherActor))
  (if (== `_as玩家` (`Controller.K2_GetPawn` (`GameplayStatics.GetPlayerController` 0)))
    (`/Engine/EditorBlueprintResources/ActorMacros.Switch Has Authority`
      (:`Remote`
        (`/Engine/EditorBlueprintResources/StandardMacros.DoOnce` false :!label _label
          (:`Completed`
            (`|ExecutionSequence`
              (:`then_0`
                (`self.投票`))
              (:`then_1`
                (`KismetSystemLibrary.Delay` 2.0)
                (goto _label :!via `Reset`)))))))))

(event `1`
  (params (Request :type "VaRestRequestJSON Object Reference"))
  (bind `_json投票` (`self.Json投票`))
  (bind _returnvalue (`VaRestRequestJSON.GetResponseContentAsString` Request false))
  (`VaRestJsonObject.DecodeJson` `_json投票` _returnvalue false)
  (set `self.票数` (`VaRestJsonObject.GetIntegerField` (`|GetArrayItem` (`VaRestJsonObject.GetObjectArrayField` (`VaRestJsonObject.GetObjectField` `_json投票` "result") "records") (`self.索引`)) "voteNum"))
  (`self.票数增加`))

(event `票数增加`
  (set `Text3DComponent.Text` (`KismetTextLibrary.Conv_IntToText` (`self.票数`)) (`self.Text3D`))
  (`self.字体动画` (/ (`KismetMathLibrary.Conv_IntToDouble` (`self.票数`)) 50.0)))

(event `字体动画`
  (params (Alpha :type "Float (single-precision)"))
  (bind _returnvalue (`KismetMathLibrary.SelectFloat` 1.0 0.0 true))
  (bind _returnvalue_2 (`KismetMathLibrary.SelectFloat` 4.0 0.0 true))
  (bind _returnvalue_3 (`SceneComponent.K2_GetComponentToWorld` (`self.Arrow`)))
  (`SceneComponent.K2_SetWorldTransform` (`self.Text3D`) (`KismetMathLibrary.TLerp` (`KismetMathLibrary.MakeTransform` (`KismetMathLibrary.MakeVector` (.x (.location _returnvalue_3)) (.y (.location _returnvalue_3)) (.z (.location _returnvalue_3))) (.rotation _returnvalue_3) (`KismetMathLibrary.MakeVector` _returnvalue _returnvalue _returnvalue)) (`KismetMathLibrary.MakeTransform` (`KismetMathLibrary.MakeVector` (.x (.location _returnvalue_3)) (.y (.location _returnvalue_3)) (.z (.location _returnvalue_3))) (.rotation _returnvalue_3) (`KismetMathLibrary.MakeVector` _returnvalue_2 _returnvalue_2 _returnvalue_2)) (select `bool` (>= Alpha 1.0) :`false` Alpha :`true` 1.0)) false false))

(event `投票`
  (set `self.json发起投票` (`|MakeJson`))
  (bind _returnvalue (`VaRestSubsystem.ConstructVaRestRequestExt` (subsystem `VaRestSubsystem`) "GET" "x_www_form_urlencoded_url"))
  (`VaRestRequestJSON.SetHeader` _returnvalue "X-Access-Token" (`/Game/game/INS.令牌` (cast `/Game/game/INS` (`GameplayStatics.GetGameInstance`) :!pure true)))
  (`VaRestRequestJSON.ProcessURL` _returnvalue (`/Game/game/函数库.附加区块链接口` (`KismetStringLibrary.Concat_StrStr` (`/Game/game/INS.API` (cast `/Game/game/INS` (`GameplayStatics.GetGameInstance`) :!pure true)) "works/voteWorks/vote?voteWorksId=" (`self.id`))))
  (add `VaRestRequestJSON.OnRequestComplete` _returnvalue (delegate `投票返回`)))

(event `投票返回`
  (params (Request :type "VaRestRequestJSON Object Reference"))
  (bind `_json发起投票` (`self.json发起投票`))
  (bind _returnvalue (`VaRestJsonObject.GetStringField` (`VaRestJsonObject.GetObjectField` `_json发起投票` "result") "verticalCoverImage"))
  (bind _returnvalue_2 (`KismetStringLibrary.IsEmpty` _returnvalue))
  (bind _returnvalue_3 (`VaRestRequestJSON.GetResponseContentAsString` Request false))
  (`VaRestJsonObject.DecodeJson` `_json发起投票` _returnvalue_3 false)
  (`/Game/game/函数库.消息提示` (select `bool` _returnvalue_2 :`false` "恭喜你获得徽章" :`true` (`KismetTextLibrary.Conv_StringToText` (`VaRestJsonObject.GetStringField` `_json发起投票` "message"))))
  (`self.获取票数`)
  (if (not _returnvalue_2)
    (`/Game/game/PLAY.生成徽章服务器` (cast `/Game/game/PLAY` (`GameplayStatics.GetPlayerController` 0) :!pure true) _returnvalue (`KismetMathLibrary.MakeVector` (.x (`self.K2_GetActorLocation`)) (+ (.y (`self.K2_GetActorLocation`)) 80.0) (+ (.z (`self.K2_GetActorLocation`)) 30.0)))))

(fn `UserConstructionScript`
  (`self.字体动画` (`self.Alpha`)))