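; Decoration actor for a badge that appears with a downloaded image and a spin.
; The construction script gives the Cube a dynamic instance of a transition material.
; On BeginPlay it downloads the image from a URL and, on success, sets it as the material texture.
; A reversed timeline then drives the transition parameter, while a second, slightly delayed timeline yaws the actor through three full turns.
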(event `self.ReceiveBeginPlay`
  (bind `_动态材质实例` (`self.动态材质实例`))
  (bind _texture (`/Game/game/蓝图宏库.图片下载` (`self.图片链接`))
    (:`On Success`
      (`MaterialInstanceDynamic.SetTextureParameterValue` `_动态材质实例` "贴图" _texture)
      (`|ExecutionSequence`
        (:`then_0`
          (bind (_direction `_新建轨道_0`) (`Timeline|时间轴_0` :!via `ReverseFromEnd`)
            (:`Update`
              (`MaterialInstanceDynamic.SetScalarParameterValue` `_动态材质实例` "过渡" (`KismetMathLibrary.Lerp` 0.8 1.2 `_新建轨道_0`)))))
        (:`then_1`
          (`KismetSystemLibrary.Delay` 0.4)
          (bind (_direction_2 `_新建轨道_0_2`) (`Timeline|时间轴_1` :!via `PlayFromStart`)
            (:`Update`
              (`self.K2_SetActorRotation` (`KismetMathLibrary.MakeRotator` 0.0 0.0 (`KismetMathLibrary.Lerp` 0.0 1080.0 `_新建轨道_0_2`))))))))))

(fn `UserConstructionScript`
  (bind _returnvalue (`PrimitiveComponent.CreateDynamicMaterialInstance` (`self.Cube`) 0 "/Game/ZY/材质/材质实例/过渡材质实例.过渡材质实例" "None"))
  (set `self.动态材质实例` _returnvalue))