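; 音效播放盒 is a trigger box actor that plays a configurable 2D sound when a player character (玩家) overlaps it.
; The overlap runs only on the Remote authority branch, so authority instances stay silent.
; An option limits playback to the pawn of the local first player controller; otherwise any player triggers it.
; Each mode has its own DoOnce gate, reset after a configurable delay unless play-once is set.
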(event `self.Box.OnComponentBeginOverlap`
  (params (OverlappedComponent :type "PrimitiveComponent Object Reference") (OtherActor :type "Actor Object Reference") (OtherComp :type "PrimitiveComponent Object Reference") (OtherBodyIndex :type Integer) (bFromSweep :type Boolean) (SweepResult :type "HitResult Structure (by ref)"))
  (`/Engine/EditorBlueprintResources/ActorMacros.Switch Has Authority`
    (:`Remote`
      (bind `_as玩家` (cast `/Game/game/玩家` OtherActor))
      (if (`self.是自己控制的玩家`)
        (if (== `_as玩家` (`Controller.K2_GetPawn` (`GameplayStatics.GetPlayerController` 0)))
          (`/Engine/EditorBlueprintResources/StandardMacros.DoOnce` false :!label _label
            (:`Completed`
              (`GameplayStatics.PlaySound2D` (`self.播放的音效`) 1.0 1.0 0.0 null null)
              (if (not (`self.是否只播放一次`))
                (`KismetSystemLibrary.Delay` (`self.触发间隔`))
                (goto _label :!via `Reset`)))))
        (else
          (`/Engine/EditorBlueprintResources/StandardMacros.DoOnce` false :!label _label_2
            (:`Completed`
              (`GameplayStatics.PlaySound2D` (`self.播放的音效`) 1.0 1.0 0.0 null null)
              (if (not (`self.是否只播放一次`))
                (`KismetSystemLibrary.Delay` (`self.触发间隔`))
                (goto _label_2 :!via `Reset`)))))))))

(fn `UserConstructionScript`)