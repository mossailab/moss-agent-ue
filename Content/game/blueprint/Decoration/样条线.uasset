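; Decoration spline Blueprint that lays a mesh along an editable spline.
; The Construction Script adds one SplineMeshComponent per pair of adjacent points, matching local positions and tangents and applying the forward axis and scale.
; The SplineMesh function is empty, with disconnected logic for distance-stepped segments, left/right side models and procedural mesh conversion that never runs.
; GetLocationTangente and ClearSplinemeshComponent serve only that unused logic.
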(fn `Clear Splinemesh Component`
  (bind _splinemeshn (`self.SplineMeshN`))
  (for _array_element _splinemeshn
    (`ActorComponent.K2_DestroyComponent` _array_element))
  (`KismetArrayLibrary.Array_Clear` _splinemeshn))

(fn `GetLocationTangente`
  (params (length1 :type "Float (double-precision)") (step1 :type "Float (double-precision)") (Spline1 :type "SplineComponent Object Reference"))
  (returns (startPos :type "Vector Structure") (startTangent :type "Vector Structure") (endPos :type "Vector Structure") (endTangent :type "Vector Structure"))
  (return (`SplineComponent.GetLocationAtDistanceAlongSpline` Spline1 (- length1 step1) "Local") (`SplineComponent.GetTangentAtDistanceAlongSpline` Spline1 (- length1 step1) "Local") (`SplineComponent.GetLocationAtDistanceAlongSpline` Spline1 length1 "Local") (`SplineComponent.GetTangentAtDistanceAlongSpline` Spline1 length1 "Local")))

(fn `SplineMesh`
  (locals (lengthT1 :type "Float (double-precision)") (SplineMesh1 :type "SplineMeshComponent Object Reference") (SplineMeshParams1 :type "Array of  Structure")))

(fn `UserConstructionScript`
  (bind _spline (`self.Spline`))
  (bind _scale (`self.Scale`))
  (for _index (range (+ (- (`SplineComponent.GetNumberOfSplinePoints` (`self.Spline`)) 2) 1))
    (bind _returnvalue (`AddComponent|NODE_AddSplineMeshComponent-3`))
    (`StaticMeshComponent.SetStaticMesh` _returnvalue (`self.Mesh`))
    (`SplineMeshComponent.SetForwardAxis` _returnvalue (`self.ForwartAxis`) true)
    (bind (_location _tangent) (`SplineComponent.GetLocationAndTangentAtSplinePoint` _spline _index "Local"))
    (bind (_location_2 _tangent_2) (`SplineComponent.GetLocationAndTangentAtSplinePoint` _spline (+ _index 1) "Local"))
    (`SplineMeshComponent.SetStartAndEnd` _returnvalue _location _tangent _location_2 _tangent_2 true)
    (`SplineMeshComponent.SetStartScale` _returnvalue _scale true)
    (`SplineMeshComponent.SetEndScale` _returnvalue _scale true)))