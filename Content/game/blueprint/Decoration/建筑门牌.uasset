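; Building nameplate decoration actor that displays the blockchain token ID, name and contract address of an architecture work.
; On clients only, ten seconds after BeginPlay, it sends a VaRest GET using the game instance's API base and token, keyed by its island index (索引).
; The completion callback decodes the JSON and fills the text fields from the first record, splitting the contract address across two lines.
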(event `self.ReceiveBeginPlay`
  (bind _asins (cast `/Game/game/INS` (`GameplayStatics.GetGameInstance`) :!pure true))
  (`/Engine/EditorBlueprintResources/ActorMacros.Switch Has Authority`
    (:`Remote`
      (`KismetSystemLibrary.Delay` 10.0)
      (set `self.门牌json` (`|MakeJson`))
      (bind _returnvalue (`VaRestSubsystem.ConstructVaRestRequestExt` (subsystem `VaRestSubsystem`) "GET" "json"))
      (`VaRestRequestJSON.SetHeader` _returnvalue "X-Access-Token" (`/Game/game/INS.令牌` _asins))
      (`VaRestRequestJSON.ProcessURL` _returnvalue (`/Game/game/函数库.附加区块链接口` (`KismetStringLibrary.Concat_StrStr` (`/Game/game/INS.API` _asins) "works/works/list?islandSubstanceTypeCode=architecture_01&islandCode=" (`self.索引`) "&noMint=false")))
      (add `VaRestRequestJSON.OnRequestComplete` _returnvalue (delegate `IP结果`)))))

(event `IP结果`
  (params (Request :type "VaRestRequestJSON Object Reference"))
  (bind `_门牌json` (`self.门牌json`))
  (bind _output (`|GetArrayItem` (`VaRestJsonObject.GetObjectArrayField` (`VaRestJsonObject.GetObjectField` `_门牌json` "result") "records")))
  (bind _returnvalue (`VaRestJsonObject.GetStringField` _output "contractAddress"))
  (bind _returnvalue_2 (`VaRestRequestJSON.GetResponseContentAsString` Request false))
  (`VaRestJsonObject.DecodeJson` `_门牌json` _returnvalue_2 false)
  (set `Text3DComponent.Text` (`KismetTextLibrary.Conv_StringToText` (`KismetStringLibrary.Concat_StrStr` "TOKEN ID:" (`VaRestJsonObject.GetStringField` _output "tokenId"))) (`self.ID`))
  (set `Text3DComponent.Text` (`KismetTextLibrary.Conv_StringToText` (`VaRestJsonObject.GetStringField` _output "name")) (`self.名称`))
  (set `Text3DComponent.Text` (`KismetTextLibrary.Conv_StringToText` (`KismetStringLibrary.Concat_StrStr` "合约地址：" (`KismetStringLibrary.GetSubstring` _returnvalue 0 23))) (`self.合约地址`))
  (set `Text3DComponent.Text` (`KismetTextLibrary.Conv_StringToText` (`KismetStringLibrary.GetSubstring` _returnvalue 23 99)) (`self.合约地址1`)))

(fn `UserConstructionScript`)