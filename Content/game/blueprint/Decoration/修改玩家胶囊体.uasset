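; Decoration trigger actor that changes the capsule size of a player (玩家) entering its Box.
; On begin overlap it casts to 玩家 and calls the 服务器 (server) event, which relays to the 组播 (multicast) event.
; That event sets capsule half height (半高) and radius (半径), skipping either when zero.
; Nothing restores the original size on leaving.
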(event `服务器`
  (params (`玩家` :type "/Game/game/玩家 Object Reference"))
  (`self.组播` `玩家`))

(event `组播`
  (params (`玩家` :type "/Game/game/玩家 Object Reference"))
  (bind _capsulecomponent (`Character.CapsuleComponent` `玩家`))
  (bind `_半径` (`self.半径`))
  (bind `_半高` (`self.半高`))
  (`|ExecutionSequence`
    (:`then_0`
      (if (not (== `_半高` 0.0))
        (`CapsuleComponent.SetCapsuleHalfHeight` _capsulecomponent `_半高` true)))
    (:`then_1`
      (if (not (== `_半径` 0.0))
        (`CapsuleComponent.SetCapsuleRadius` _capsulecomponent `_半径` true)))))

(event `self.Box.OnComponentBeginOverlap`
  (params (OverlappedComponent :type "PrimitiveComponent Object Reference") (OtherActor :type "Actor Object Reference") (OtherComp :type "PrimitiveComponent Object Reference") (OtherBodyIndex :type Integer) (bFromSweep :type Boolean) (SweepResult :type "HitResult Structure (by ref)"))
  (bind `_as玩家` (cast `/Game/game/玩家` OtherActor))
  (`self.服务器` `_as玩家`))

(fn `UserConstructionScript`)