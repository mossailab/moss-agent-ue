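; Escalator step component (电梯部件) that loops a stair mesh along the Spline of its parent 电梯 actor.
; 时间轴_0 drives spline position, staggered by 索引 times three seconds.
; On finishing, two timelines sink the mesh, then raise it at the spline start before restarting in the 反向 direction.
; BeginPlay copies 反向 from the parent only after starting movement, so the first pass uses the component's prior value.
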(event `self.ReceiveBeginPlay`
  (`self.1`)
  (bind `_as电梯` (cast `/Game/game/blueprint/Decoration/电梯` (`self.GetParentActor`)))
  (set `self.反向` (`/Game/game/blueprint/Decoration/电梯.反向` `_as电梯`)))

(event `1`
  (bind _a (`self.A`))
  (bind _a_2 (`self.A`))
  (bind `_as电梯` (cast `/Game/game/blueprint/Decoration/电梯` (`self.GetParentActor`) :!label _label))
  (set `self.Spline` (`/Game/game/blueprint/Decoration/电梯.Spline` `_as电梯`))
  (`|ExecutionSequence`
    (:`then_0`
      (bind (_direction `_新建轨道_0`) (`Timeline|时间轴_0` :`NewTime` (* (`KismetMathLibrary.Conv_IntToDouble` (`self.索引`)) 3.0) :!via `SetNewTime` :!label _label_2)
        (:`Update`
          (`self.2` (`SplineComponent.GetLocationAtTime` (`self.Spline`) `_新建轨道_0` "World" false)))
        (:`Finished`
          (set `self.A` (`SceneComponent.K2_GetComponentLocation` (`self.Linear_Stair_StaticMesh`)))
          (bind (_direction_2 `_新建轨道_0_2`) (`Timeline|时间轴_1` :!via `PlayFromStart`)
            (:`Update`
              (`self.2` (`KismetMathLibrary.VLerp` _a (`KismetMathLibrary.MakeVector` (.x _a) (.y _a) (- (.z _a) 20.0)) `_新建轨道_0_2`)))
            (:`Finished`
              (set `self.A` (`SplineComponent.GetLocationAtTime` (`self.Spline`) 0.0 "World" false))
              (bind (_direction_3 `_新建轨道_0_3`) (`Timeline|时间轴_2` :!via `PlayFromStart`)
                (:`Update`
                  (`self.2` (`KismetMathLibrary.VLerp` (`KismetMathLibrary.MakeVector` (.x _a_2) (.y _a_2) (- (.z _a_2) 20.0)) _a_2 `_新建轨道_0_3`)))
                (:`Finished`
                  (if (`self.反向`)
                    (goto _label_2 :!via `ReverseFromEnd`)
                    (else
                      (goto _label_2 :!via `PlayFromStart`))))))))))
    (:`then_1`
      (if (`self.反向`)
        (goto _label_2 :!via `Reverse`)
        (else
          (goto _label_2))))))

(event `11`
  (goto _label))

(event `2`
  (params (NewParam :type "Vector Structure"))
  (`SceneComponent.K2_SetWorldLocation` (`self.Linear_Stair_StaticMesh`) NewParam false false))

(fn `UserConstructionScript`)