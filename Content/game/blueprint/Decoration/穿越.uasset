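; Decorative two-way portal (穿越) that teleports players who walk into trigger A or B and plays a looping media source from BeginPlay.
; On overlap, only the authority acts, calling the player's 传送自身 with that trigger's target location and rotation.
; Players flagged 已进行传送 are skipped.
; Only trigger A sets the teleport-into-air option (传送到空中).
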(event `self.ReceiveBeginPlay`
  (bind `_播放器` (`self.播放器`))
  (`MediaPlayer.OpenSource` `_播放器` "/Game/game/视频媒体/tp106/TP106_1.TP106_1")
  (`MediaPlayer.Play` `_播放器`)
  (`MediaPlayer.SetLooping` `_播放器` true))

(event `self.A.OnComponentBeginOverlap`
  (params (OverlappedComponent :type "PrimitiveComponent Object Reference") (OtherActor :type "Actor Object Reference") (OtherComp :type "PrimitiveComponent Object Reference") (OtherBodyIndex :type Integer) (bFromSweep :type Boolean) (SweepResult :type "HitResult Structure (by ref)"))
  (bind `_as玩家` (cast `/Game/game/玩家` OtherActor))
  (`/Engine/EditorBlueprintResources/ActorMacros.Switch Has Authority`
    (:`Authority`
      (if (not (`/Game/game/玩家.已进行传送` `_as玩家`))
        (`/Game/game/玩家.传送自身` `_as玩家` (.location (`SceneComponent.K2_GetComponentToWorld` (`self.A传送目标位置`))) (.rotation (`SceneComponent.K2_GetComponentToWorld` (`self.A传送目标位置`))) null true)))))

(event `self.B.OnComponentBeginOverlap`
  (params (OverlappedComponent :type "PrimitiveComponent Object Reference") (OtherActor :type "Actor Object Reference") (OtherComp :type "PrimitiveComponent Object Reference") (OtherBodyIndex :type Integer) (bFromSweep :type Boolean) (SweepResult :type "HitResult Structure (by ref)"))
  (bind `_as玩家` (cast `/Game/game/玩家` OtherActor))
  (`/Engine/EditorBlueprintResources/ActorMacros.Switch Has Authority`
    (:`Authority`
      (if (not (`/Game/game/玩家.已进行传送` `_as玩家`))
        (`/Game/game/玩家.传送自身` `_as玩家` (.location (`SceneComponent.K2_GetComponentToWorld` (`self.B传送目标位置`))) (.rotation (`SceneComponent.K2_GetComponentToWorld` (`self.B传送目标位置`))) null false)))))

(fn `UserConstructionScript`)