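; Airdrop actor that drops a treasure crate at a target position and opens it on landing.
; On BeginPlay the authority calls 初始组播, which sets the child 宝藏内容's image and lerps the actor to the target by timeline.
; A second timeline lowers Cube with sweep while raising FallingCrate by a frame-rate-based step.
; A blocking hit or timeline end triggers, once, the crate montage and, after a delay, 打开宝箱.
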(event `self.ReceiveTick`
  (params (DeltaSeconds :type "Float (single-precision)"))
  (set `self.帧数` (/ 1.0 DeltaSeconds)))

(event `初始组播`
  (bind _fallingcrate (`self.FallingCrate`))
  (bind (_returnvalue_x _returnvalue_y _returnvalue_z) (`KismetMathLibrary.BreakVector` (`SceneComponent.K2_GetComponentLocation` _fallingcrate)))
  (`/Game/game/blueprint/Decoration/宝藏内容.设置图像` (cast `/Game/game/blueprint/Decoration/宝藏内容` (`ChildActorComponent.ChildActor` (`self.ChildActor`)) :!pure true) (`self.图片链接`))
  (`|PlayMontage` (`self.FallingCrate`)
    (:`then`
      (set `self.A` (`self.K2_GetActorLocation`))
      (bind (_direction `_新建轨道_0`) (`Timeline|下落动画` :!via `PlayFromStart`)
        (:`Update`
          (`self.K2_SetActorLocation` (`KismetMathLibrary.VLerp` (`self.A`) (`self.目标位置`) `_新建轨道_0`) true))
        (:`Finished`
          (set `self.B` (`SceneComponent.K2_GetComponentLocation` (`self.Cube`)))
          (bind (_direction_2 `_新建轨道_0_2`) (`Timeline|宝箱时间轴` :!via `PlayFromStart`)
            (:`Update`
              (`SceneComponent.K2_SetWorldLocation` _fallingcrate (`KismetMathLibrary.MakeVector` _returnvalue_x _returnvalue_y (+ _returnvalue_z (* (`self.帧数`) 0.5))) false false)
              (bind _sweephitresult (`SceneComponent.K2_SetWorldLocation` (`self.Cube`) (`KismetMathLibrary.VLerp` (`self.B`) (`KismetMathLibrary.MakeVector` (.x (`self.目标位置`)) (.y (`self.目标位置`)) (- (.z (`self.目标位置`)) 500.0)) `_新建轨道_0_2`) true false))
              (bind (_bblockinghit _binitialoverlap _time _distance _location _impactpoint _normal _impactnormal _physmat _hitactor) (`GameplayStatics.BreakHitResult` _sweephitresult))
              (if _bblockinghit
                (`KismetSystemLibrary.PrintString` (`KismetSystemLibrary.GetDisplayName` _hitactor))
                (`/Engine/EditorBlueprintResources/StandardMacros.DoOnce` false :!label _label
                  (:`Completed`
                    (`|PlayMontage` (`self.箱子`)
                      (:`then`
                        (`KismetSystemLibrary.Delay` 1.0)
                        (bind `_as宝藏内容` (cast `/Game/game/blueprint/Decoration/宝藏内容` (`ChildActorComponent.ChildActor` (`self.ChildActor`))))
                        (`/Game/game/blueprint/Decoration/宝藏内容.打开宝箱` `_as宝藏内容`)))))))
            (:`Finished`
              (goto _label))))))))

(event `self.ReceiveBeginPlay`
  (`/Engine/EditorBlueprintResources/ActorMacros.Switch Has Authority`
    (:`Authority`
      (`self.初始服务器`))))

(event `初始服务器`
  (`self.初始组播`))

(fn `UserConstructionScript`)