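; Server-jump decoration actor (服务器跳转) that moves the player to another level when their pawn overlaps its Sphere.
; A DoOnce gate plays a pickup sound, then opens the level named in 关卡, or calls the PLAY controller's 全局加载空间 as main level if that is empty.
; A 询问控件 confirmation dialog, whose callback would continue the jump or reset the gate, is disconnected, so the jump happens immediately.
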(event `self.Sphere.OnComponentBeginOverlap`
  (params (OverlappedComponent :type "PrimitiveComponent Object Reference") (OtherActor :type "Actor Object Reference") (OtherComp :type "PrimitiveComponent Object Reference") (OtherBodyIndex :type Integer) (bFromSweep :type Boolean) (SweepResult :type "HitResult Structure (by ref)"))
  (bind `_关卡` (`self.关卡`))
  (if (== OtherActor (`GameplayStatics.GetPlayerPawn` 0))
    (`/Engine/EditorBlueprintResources/StandardMacros.DoOnce` false :!label _label
      (:`Completed`
        (`GameplayStatics.PlaySound2D` "/Game/game/音效/InterdimensionalInterfaceVol1/CUE/开舱门/CUE_Get_Object_02_Cue.CUE_Get_Object_02_Cue" 1.0 1.0 0.0 null null :!label _label_2)
        (if (`KismetStringLibrary.IsEmpty` `_关卡`)
          (`/Game/game/PLAY.全局加载空间` (cast `/Game/game/PLAY` (`GameplayStatics.GetPlayerController` 0) :!pure true) "" "" false false true "服务器跳转actor")
          (else
            (`GameplayStatics.OpenLevel` (`KismetStringLibrary.Conv_StringToName` `_关卡`))))))))

(event `自定义事件`
  (params (`为确定` :type Boolean))
  (if `为确定`
    (goto _label_2)
    (else
      (goto _label :!via `Reset`))))

(fn `UserConstructionScript`)