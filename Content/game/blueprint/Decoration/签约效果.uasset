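; Decoration Blueprint for a signing effect (签约效果): a globe sphere that spins, rises and bursts on BeginPlay.
; One timeline lifts and scales the sphere while ramping spin and Niagara particle parameters.
; It then spawns an explosion, hides the sphere and enables a particle model, as a second timeline slows spin, lowers the sphere and drives another transition.
; Tick applies rotation and feeds sphere height to Niagara.
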(event `self.ReceiveBeginPlay`
  (`self.地球飞起`))

(event `地球飞起`
  (bind _3 (`self.3`))
  (bind _4 (`self.4`))
  (bind _sphere (`self.Sphere`))
  (bind _a (`self.A`))
  (bind _location (.location (`self.A`)))
  (set `self.A` (`SceneComponent.K2_GetComponentToWorld` (`self.Sphere`)))
  (bind (_direction `_新建轨道_0`) (`Timeline|时间轴_0` :!via `PlayFromStart`)
    (:`Update`
      (bind (_returnvalue_location _returnvalue_rotation _returnvalue_scale) (`KismetMathLibrary.BreakTransform` (`KismetMathLibrary.TLerp` _a (`KismetMathLibrary.MakeTransform` (`KismetMathLibrary.MakeVector` (.x (.location _a)) (.y (.location _a)) (+ (.z (.location _a)) 500.0)) (struct) (`KismetMathLibrary.Conv_DoubleToVector` (`KismetMathLibrary.SelectFloat` 3.0 3.0 true))) `_新建轨道_0`)))
      (`SceneComponent.K2_SetWorldLocation` _sphere _returnvalue_location false false)
      (`SceneComponent.SetWorldScale3D` _sphere _returnvalue_scale)
      (set `self.旋转速度` (`KismetMathLibrary.Lerp` 0.0 30.0 `_新建轨道_0`))
      (`FXSystemComponent.SetIntParameter` _3 "生成数量" (`KismetMathLibrary.FTrunc` (`KismetMathLibrary.Lerp` 500.0 20000.0 `_新建轨道_0`)))
      (`FXSystemComponent.SetFloatParameter` _3 "旋转力" (`KismetMathLibrary.Lerp` 500.0 5000.0 `_新建轨道_0`))
      (`FXSystemComponent.SetFloatParameter` _4 "过度" (`KismetMathLibrary.Lerp` 0.0 0.5 `_新建轨道_0`))
      (`FXSystemComponent.SetFloatParameter` _4 "生成范围" (`KismetMathLibrary.Lerp` 20.0 8.0 `_新建轨道_0`)))
    (:`Finished`
      (`FXSystemComponent.SetIntParameter` (`self.3`) "生成数量" 0)
      (`self.爆炸`)
      (`SceneComponent.SetVisibility` (`self.Sphere`) false false)
      (`FXSystemComponent.SetBoolParameter` (`self.4`) "开启模型" true)
      (bind (_direction_2 `_新建轨道_0_2`) (`Timeline|时间轴_1` :!via `PlayFromStart`)
        (:`Update`
          (set `self.旋转速度` (`KismetMathLibrary.Lerp` 30.0 1.0 `_新建轨道_0_2`))
          (`FXSystemComponent.SetFloatParameter` (`self.5`) "过度" (`KismetMathLibrary.Lerp` 0.0 1.0 `_新建轨道_0_2`))
          (`SceneComponent.K2_SetWorldLocation` (`self.Sphere`) (`KismetMathLibrary.VLerp` (`KismetMathLibrary.MakeVector` (.x _location) (.y _location) (+ (.z _location) 500.0)) _location `_新建轨道_0_2`) false false))))))

(event `self.ReceiveTick`
  (params (DeltaSeconds :type "Float (single-precision)"))
  (bind `_旋转速度` (`self.旋转速度`))
  (`SceneComponent.K2_AddWorldRotation` (`self.Sphere`) (`KismetMathLibrary.MakeRotator` 0.0 0.0 `_旋转速度`) false false)
  (if (> `_旋转速度` 0.0)
    (`FXSystemComponent.SetVectorParameter` (`self.4`) "输入位置" (`KismetMathLibrary.MakeVector` 0.0 0.0 (.z (.location (`SceneComponent.GetRelativeTransform` (`self.Sphere`))))))))

(event `爆炸`
  (bind _returnvalue (`NiagaraFunctionLibrary.SpawnSystemAtLocation` "/Game/game/特效/NiagaraAbstractSpace/Effects/1.1" (`SceneComponent.K2_GetComponentLocation` (`self.Sphere`))))
  (set `self.NewVar` _returnvalue)
  (bind (_direction `_新建轨道_2`) (`Timeline|时间轴` :!via `PlayFromStart`)
    (:`Update`
      (bind _newvar (`self.NewVar`)
        (:`then`
          (`FXSystemComponent.SetFloatParameter` _newvar "1" (`KismetMathLibrary.Lerp` 1.0 -3.0 `_新建轨道_2`)))
        (:`else`)))))

(fn `UserConstructionScript`
  (`FXSystemComponent.SetFloatParameter` (`self.4`) "生成范围" 20.0))