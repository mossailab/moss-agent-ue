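; Level-transition terminal that, on its first overlap with the 模特 character, disables player input and loads the GW_zhiying level after a timed effect.
; The construction script creates two dynamic UI materials on the mesh, whose diffuse texture parameter is set on trigger as the 3D text appears.
; A slowed timeline ramps the PC_Control material parameter collection while two sound cues play in sequence, then opens the level when finished.
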(event `self.Sphere.OnComponentBeginOverlap`
  (params (OverlappedComponent :type "PrimitiveComponent Object Reference") (OtherActor :type "Actor Object Reference") (OtherComp :type "PrimitiveComponent Object Reference") (OtherBodyIndex :type Integer) (bFromSweep :type Boolean) (SweepResult :type "HitResult Structure (by ref)"))
  (bind `_as模特` (cast `/Game/game/blueprint/nr/模特` OtherActor))
  (`/Engine/EditorBlueprintResources/StandardMacros.DoOnce` false
    (:`Completed`
      (`self.DisableInput` `_as模特` (`GameplayStatics.GetPlayerController` 0))
      (`MaterialInstanceDynamic.SetTextureParameterValue` (`self.A`) "diffuse" null)
      (`MaterialInstanceDynamic.SetTextureParameterValue` (`self.B`) "diffuse" null)
      (`SceneComponent.SetVisibility` (`self.Text3D`) true false)
      (`KismetMaterialLibrary.SetScalarParameterValue` "/Game/chensongxin/场景溶解/PC_Control.PC_Control" "divide" 3000.0)
      (`TimelineComponent.SetPlayRate` (`self.时间轴`) 0.1)
      (`|ExecutionSequence`
        (:`then_0`
          (bind (_direction `_新建轨道_0`) (`Timeline|时间轴` :!via `PlayFromStart`)
            (:`Update`
              (`KismetMaterialLibrary.SetScalarParameterValue` "/Game/chensongxin/场景溶解/PC_Control.PC_Control" "aomount" (`KismetMathLibrary.Lerp` 0.0 5.0 `_新建轨道_0`)))
            (:`Finished`
              (`GameplayStatics.OpenLevel` "GW_zhiying"))))
        (:`then_1`
          (`GameplayStatics.PlaySound2D` "/Game/game/音效/InterdimensionalInterfaceVol1/CUE/开舱门/CUE_Get_Object_10_Cue.CUE_Get_Object_10_Cue" 1.0 1.0 0.0 null null)
          (`KismetSystemLibrary.Delay` 2.5)
          (`GameplayStatics.PlaySound2D` "/Game/game/音效/InterdimensionalInterfaceVol1/CUE/开舱门/CUE_Get_Object_02_Cue.CUE_Get_Object_02_Cue" 1.0 1.0 0.0 null null))))))

(fn `UserConstructionScript`
  (bind _staticmesh (`self.StaticMesh`))
  (bind _returnvalue (`PrimitiveComponent.CreateDynamicMaterialInstance` _staticmesh 0 "/Game/ZY/静态网格体/StarterBundle/ModularSci_Comm/Materials/MI_Terminal_A_UI_1.MI_Terminal_A_UI_1" "None"))
  (set `self.A` _returnvalue)
  (bind _returnvalue_2 (`PrimitiveComponent.CreateDynamicMaterialInstance` _staticmesh 2 "/Game/ZY/静态网格体/StarterBundle/ModularSci_Comm/Materials/MI_Terminal_A_UI_1B.MI_Terminal_A_UI_1B" "None"))
  (set `self.B` _returnvalue_2))