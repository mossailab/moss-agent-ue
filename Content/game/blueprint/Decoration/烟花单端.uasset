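; Decorative fireworks actor that launches randomized Niagara bursts around its position, in every level except JH1.
; On BeginPlay a DoN loop runs a configurable number of rounds, waiting an interval before each one and calling the 发射烟花 event.
; Each round spawns several effects picked at random from a template array, with random XY offset at the actor's height and random roll and pitch.
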(event `self.ReceiveBeginPlay`
  (bind _returnvalue (`GameplayStatics.GetCurrentLevelName` true))
  (if (not (== _returnvalue "JH1"))
    (`/Engine/EditorBlueprintResources/StandardMacros.Do N` (`self.生成几轮`) :!label _label
      (:`Exit`
        (`KismetSystemLibrary.Delay` (`self.每轮间隔`))
        (`self.发射烟花`)
        (goto _label)))))

(event `发射烟花`
  (bind _system_template (`self.System Template`))
  (bind `_随机范围` (`self.随机范围`))
  (bind `_随机范围_2` (`self.随机范围`))
  (bind `_随机角度` (`self.随机角度`))
  (bind _x (.x (`self.K2_GetActorLocation`)))
  (bind _y (.y (`self.K2_GetActorLocation`)))
  (bind _returnvalue (`KismetMathLibrary.RandomFloatInRange` (* `_随机角度` -1.0) `_随机角度`))
  (for _ (range 1 (+ (`self.生成数量`) 1))
    (`NiagaraFunctionLibrary.SpawnSystemAtLocation` (`|GetArrayItem` _system_template (`KismetMathLibrary.RandomIntegerInRange` 0 (- (`KismetArrayLibrary.Array_Length` _system_template) 1))) (`KismetMathLibrary.MakeVector` (`KismetMathLibrary.RandomFloatInRange` (- _x `_随机范围_2`) (+ _x `_随机范围_2`)) (`KismetMathLibrary.RandomFloatInRange` (- _y `_随机范围`) (+ _y `_随机范围`)) (.z (`self.K2_GetActorLocation`))) (`KismetMathLibrary.MakeRotator` _returnvalue _returnvalue))))

(fn `UserConstructionScript`)